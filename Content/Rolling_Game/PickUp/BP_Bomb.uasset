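; BP_Bomb is a hazard in the rolling game that damages the player's ball pawn on contact.
; On BeginPlay it plays a fuse-spark sound at its mesh location.
; When its sphere overlaps BP_Player_Pawn, it decrements health by Damage and applies a large impulse opposite the Ball component's forward vector.
; It then plays an explosion sound and destroys itself, ignoring all other actors.
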(event OnComponentBeginOverlap(Sphere)
  (params (OverlappedComponent :type Primitive%20Component%20Object%20Reference) (OtherActor :type Actor%20Object%20Reference) (OtherComp :type Primitive%20Component%20Object%20Reference) (OtherBodyIndex :type Integer) (bFromSweep :type Boolean) (SweepResult :type Hit%20Result%20Structure%20%28by%20ref%29))
  (bind _asbp_player_pawn (Utilities|Casting|CastToBP_Player_Pawn OtherActor))
  (Default|DecremetHealth _asbp_player_pawn (Variables|Default|GetDamage))
  (Physics|AddImpulse (Variables|/Game/Rolling_Game/Player/BP_Player_Pawn.BP_Player_Pawn_C|GetBall _asbp_player_pawn) (* (Math|Vector|GetForwardVector (Variables|/Game/Rolling_Game/Player/BP_Player_Pawn.BP_Player_Pawn_C|GetBall _asbp_player_pawn)) -1e+05) "None" false)
  (Audio|PlaySoundatLocation "/Game/Rolling_Game/PickUp/Textures/Explosion01.Explosion01" (Transformation|GetWorldLocation (Variables|Default|GetStaticMesh)) "0, 0, 0" 1.0 1.0 0.0 0 0 0)
  (Actor|DestroyActor))

(event EventBeginPlay
  (Audio|PlaySoundatLocation "/Game/StarterContent/Audio/Fire_Sparks01_Cue.Fire_Sparks01_Cue" (Transformation|GetWorldLocation (Variables|Default|GetStaticMesh)) "0, 0, 0" 1.0 1.0 0.0 0 0 0))

(event Collision|EventActorBeginOverlap
  (params (OtherActor :type Actor%20Object%20Reference)))

(event EventTick
  (params (DeltaSeconds :type Float%20%28single-precision%29)))

(fn ConstructionScript)