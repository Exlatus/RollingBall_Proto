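; BP_PickUps is a collectible that awards points when a BP_Player_Pawn overlaps its sphere.
; On pickup it increments the pawn's goal target count, adds score, and plays a sound and particle effect.
; A widget component, given the point value and hidden at BeginPlay, appears and plays a pickup animation.
; The mesh hides at once, while the actor is destroyed after a short delay.
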(event OnComponentBeginOverlap(Sphere)
  (params (OverlappedComponent :type Primitive%20Component%20Object%20Reference) (OtherActor :type Actor%20Object%20Reference) (OtherComp :type Primitive%20Component%20Object%20Reference) (OtherBodyIndex :type Integer) (bFromSweep :type Boolean) (SweepResult :type Hit%20Result%20Structure%20%28by%20ref%29))
  (bind _asbp_player_pawn (Utilities|Casting|CastToBP_Player_Pawn OtherActor))
  (Default|IncremetGoalTargets _asbp_player_pawn)
  (Audio|PlaySoundatLocation (Variables|Default|Getsound_play_on_destroy) (Transformation|GetWorldLocation (Variables|Default|GetStaticMesh)) "0, 0, 0" 1.0 1.0 0.0 0 0 0)
  (Default|AddScore _asbp_player_pawn (Variables|Default|GetPoints_pickup))
  (Effects|SpawnEmitteratLocation (Variables|Default|GetParticleOnPickup) (Transformation|GetActorLocation))
  (Rendering|SetVisibility (Variables|Default|GetBP_Widget) true false)
  (bind _asbp_widget (Utilities|Casting|CastToBP_Widget (UserInterface|GetUserWidgetObject (Variables|Default|GetBP_Widget))))
  (UserInterface|Animation|PlayAnimation _asbp_widget (Variables|/Game/Rolling_Game/PickUp/BP_Widget.BP_Widget_C|GetAnimationPickup _asbp_widget) 0.0 1 "Forward" 1.0 false)
  (Rendering|SetVisibility (Variables|Default|GetStaticMesh) false false)
  (Utilities|FlowControl|Delay 0.75)
  (Actor|DestroyActor))

(event EventBeginPlay
  (bind _bp_widget (Variables|Default|GetBP_Widget))
  (Rendering|SetVisibility _bp_widget false false)
  (bind _asbp_widget (Utilities|Casting|CastToBP_Widget (UserInterface|GetUserWidgetObject _bp_widget)))
  (Variables|/Game/Rolling_Game/PickUp/BP_Widget.BP_Widget_C|SetScore_value _asbp_widget (Variables|Default|GetPoints_pickup)))

(event Collision|EventActorBeginOverlap
  (params (OtherActor :type Actor%20Object%20Reference)))

(event EventTick
  (params (DeltaSeconds :type Float%20%28single-precision%29)))

(fn ConstructionScript)