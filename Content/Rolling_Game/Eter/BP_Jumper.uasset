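; BP_Jumper is a jump pad that launches the player's ball when BP_Player_Pawn hits its Button.
; The hit plays a sound and applies a velocity-change impulse to the pawn's Ball along the Button's up vector.
; A timeline offsets the Button in world Z from its BeginPlay location, with a delayed Reverse chained from the timeline's Update to return it.
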(event OnComponentHit(Button)
  (params (HitComponent :type Primitive%20Component%20Object%20Reference) (OtherActor :type Actor%20Object%20Reference) (OtherComp :type Primitive%20Component%20Object%20Reference) (NormalImpulse :type Vector :default "0, 0, 0") (Hit :type Hit%20Result%20Structure%20%28by%20ref%29))
  (bind _buttonworldlocation (Variables|Default|GetButtonWorldLocation))
  (bind (_x _y _z) (Math|Vector|BreakVector _buttonworldlocation))
  (bind _asbp_player_pawn (Utilities|Casting|CastToBP_Player_Pawn OtherActor))
  (Audio|PlaySound2D "/Engine/VREditor/Sounds/VR_open.VR_open" 1.0 1.0 0.0 0 0)
  (Physics|AddImpulse (Variables|/Game/Rolling_Game/Player/BP_Player_Pawn.BP_Player_Pawn_C|GetBall _asbp_player_pawn) (* (Math|Vector|GetUpVector (Variables|Default|GetButton)) 8e+02) "None" true)
  (bind _newtrack_0 (Timeline|JumperTimeline Play)
    (:Update
      (Transformation|SetWorldLocation (Variables|Default|GetButton) (Math|Vector|MakeVector _x _y (+ _z _newtrack_0)) false false)
      (Utilities|FlowControl|Delay 0.5)
      (Timeline|JumperTimeline Reverse))))

(event EventBeginPlay
  (Variables|Default|SetButtonWorldLocation (Transformation|GetWorldLocation (Variables|Default|GetButton))))

(fn ConstructionScript)