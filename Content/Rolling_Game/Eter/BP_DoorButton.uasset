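; Pressure-plate actor for the rolling game that moves a door while the player pawn is on the button.
; Overlapping the sphere trigger plays a sound and runs a timeline; leaving it reverses the timeline after a short delay, with a closing sound.
; Two timeline curves drive UpdateButton, which offsets the button and door vertically from world locations cached at BeginPlay.
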(event OnComponentBeginOverlap(Sphere)
  (params (OverlappedComponent :type Primitive%20Component%20Object%20Reference) (OtherActor :type Actor%20Object%20Reference) (OtherComp :type Primitive%20Component%20Object%20Reference) (OtherBodyIndex :type Integer) (bFromSweep :type Boolean) (SweepResult :type Hit%20Result%20Structure%20%28by%20ref%29))
  (Utilities|Casting|CastToBP_Player_Pawn OtherActor)
  (Audio|PlaySound2D "/Engine/VREditor/Sounds/UI/Dockable_Window_Open.Dockable_Window_Open" 1.0 1.0 0.0 0 0)
  (bind (_direction _buttonelevation _doortimeline) (Timeline|ButtonTimeline Play)
    (:Update
      (CallFunction|UpdateButton _buttonelevation _doortimeline))))

(event OnComponentEndOverlap(Sphere)
  (params (OverlappedComponent :type Primitive%20Component%20Object%20Reference) (OtherActor :type Actor%20Object%20Reference) (OtherComp :type Primitive%20Component%20Object%20Reference) (OtherBodyIndex :type Integer))
  (Utilities|Casting|CastToBP_Player_Pawn OtherActor)
  (Utilities|FlowControl|Delay 0.2)
  (Audio|PlaySound2D "/Engine/VREditor/Sounds/UI/Dockable_Window_Close.Dockable_Window_Close" 1.0 1.0 0.0 0 0)
  (bind (_direction _buttonelevation _doortimeline) (Timeline|ButtonTimeline Reverse)
    (:Update
      (CallFunction|UpdateButton _buttonelevation _doortimeline))))

(event EventBeginPlay
  (Variables|Default|SetButtonWorldLocation (Transformation|GetWorldLocation (Variables|Default|GetButton_Little)))
  (Variables|Default|SetDoorWorldLocation (Transformation|GetWorldLocation (Variables|Default|GetDoor))))

(fn ConstructionScript)

(fn UpdateButton
  (params (UpdateButton :type Float%20%28single-precision%29) (UpdateDoor :type Float%20%28single-precision%29))
  (bind _buttonworldlocation (Variables|Default|GetButtonWorldLocation))
  (bind _doorworldlocation (Variables|Default|GetDoorWorldLocation))
  (bind (_x _y _z) (Math|Vector|BreakVector _doorworldlocation))
  (bind (_x_2 _y_2 _z_2) (Math|Vector|BreakVector _buttonworldlocation))
  (Utilities|FlowControl|Sequence
    (:then_0
      (Transformation|SetWorldLocation (Variables|Default|GetButton_Little) (Math|Vector|MakeVector _x_2 _y_2 (+ _z_2 UpdateButton)) false false))
    (:then_1
      (Transformation|SetWorldLocation (Variables|Default|GetDoor) (Math|Vector|MakeVector _x _y (+ _z UpdateDoor)) false false))))