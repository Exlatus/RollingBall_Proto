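; BP_Booster is a boost button that propels the rolling player ball when it enters the sphere trigger.
; Overlap plays a sound and runs a timeline that offsets the button's height; leaving plays another sound and reverses it.
; Every timeline update, in both directions, also adds an impulse along the ball's forward vector and doubles the pawn's TorqueBall, so torque compounds with no reset here.
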(event OnComponentBeginOverlap(Sphere)
  (params (OverlappedComponent :type Primitive%20Component%20Object%20Reference) (OtherActor :type Actor%20Object%20Reference) (OtherComp :type Primitive%20Component%20Object%20Reference) (OtherBodyIndex :type Integer) (bFromSweep :type Boolean) (SweepResult :type Hit%20Result%20Structure%20%28by%20ref%29))
  (bind _buttonworldlocation (Variables|Default|GetButtonWorldLocation))
  (bind (_x _y _z) (Math|Vector|BreakVector _buttonworldlocation))
  (bind _asbp_player_pawn (Utilities|Casting|CastToBP_Player_Pawn OtherActor))
  (Variables|Default|SetrefBP_Player_Pawn _asbp_player_pawn)
  (Audio|PlaySound2D "/Engine/EditorSounds/GamePreview/EjectFromPlayer.EjectFromPlayer" 1.0 1.0 0.0 0 0)
  (bind _burronboostertimeline (Timeline|ButtonBoostTimeline Play)
    (:Update
      (Transformation|SetWorldLocation (Variables|Default|GetBoostButton) (Math|Vector|MakeVector _x _y (+ _z _burronboostertimeline)) false false)
      (Physics|AddImpulse (Variables|/Game/Rolling_Game/Player/BP_Player_Pawn.BP_Player_Pawn_C|GetBall (Variables|Default|GetrefBP_Player_Pawn)) (* (Math|Vector|GetForwardVector (Variables|/Game/Rolling_Game/Player/BP_Player_Pawn.BP_Player_Pawn_C|GetBall (Variables|Default|GetrefBP_Player_Pawn))) 5e+02) "None" false)
      (Variables|/Game/Rolling_Game/Player/BP_Player_Pawn.BP_Player_Pawn_C|SetTorque_Ball (Variables|Default|GetrefBP_Player_Pawn) (* (Variables|/Game/Rolling_Game/Player/BP_Player_Pawn.BP_Player_Pawn_C|GetTorque_Ball (Variables|Default|GetrefBP_Player_Pawn)) 2.0)))))

(event OnComponentEndOverlap(Sphere)
  (params (OverlappedComponent :type Primitive%20Component%20Object%20Reference) (OtherActor :type Actor%20Object%20Reference) (OtherComp :type Primitive%20Component%20Object%20Reference) (OtherBodyIndex :type Integer))
  (bind _buttonworldlocation (Variables|Default|GetButtonWorldLocation))
  (bind _refbp_player_pawn (Variables|Default|GetrefBP_Player_Pawn))
  (bind (_x _y _z) (Math|Vector|BreakVector _buttonworldlocation))
  (bind _ball (Variables|/Game/Rolling_Game/Player/BP_Player_Pawn.BP_Player_Pawn_C|GetBall _refbp_player_pawn))
  (Utilities|Casting|CastToBP_Player_Pawn OtherActor)
  (Audio|PlaySound2D "/Engine/VREditor/Sounds/UI/Object_PickUp.Object_PickUp" 1.0 1.0 0.0 0 0)
  (bind _burronboostertimeline (Timeline|ButtonBoostTimeline Reverse)
    (:Update
      (Transformation|SetWorldLocation (Variables|Default|GetBoostButton) (Math|Vector|MakeVector _x _y (+ _z _burronboostertimeline)) false false)
      (Physics|AddImpulse _ball (* (Math|Vector|GetForwardVector _ball) 5e+02) "None" false)
      (Variables|/Game/Rolling_Game/Player/BP_Player_Pawn.BP_Player_Pawn_C|SetTorque_Ball _refbp_player_pawn (* (Variables|/Game/Rolling_Game/Player/BP_Player_Pawn.BP_Player_Pawn_C|GetTorque_Ball _refbp_player_pawn) 2.0)))))

(event EventBeginPlay
  (Variables|Default|SetButtonWorldLocation (Transformation|GetWorldLocation (Variables|Default|GetBoostButton))))

(fn ConstructionScript)